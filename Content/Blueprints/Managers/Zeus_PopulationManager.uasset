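; Population manager actor that spawns immigrants at its own transform to fill free housing in the city.
; Each tick, when no Zeus_Immigrant exists and housing remains, it spawns one, so only one immigrant is in transit at a time.
; Remaining housing is total MaxResidents across all Zeus_Building actors minus current residents and homeless immigrants, recounted through GetAllActorsOfClass queries on every check.
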(event EventBeginPlay)

(event Collision|EventActorBeginOverlap
  (params (OtherActor :type Actor%20Object%20Reference)))

(event EventTick
  (params (DeltaSeconds :type Float%20%28single-precision%29))
  (bind _returnvalue (CallFunction|HomelessPopulation))
  (if (== _returnvalue 0)
    (bind _total_housing (CallFunction|RemainingHousing))
    (if (> _total_housing 0)
      (CallFunction|SpawnImmigrant))))

(fn ConstructionScript)

(fn SpawnImmigrant
  (Game|SpawnActorfromClass "/Game/Blueprints/Pawns/Zeus_Immigrant.Zeus_Immigrant_C" (Transformation|GetActorTransform) "Undefined" 0 0))

(fn HousingCapacity
  (bind _outactors (Actor|GetAllActorsOfClass "/Game/Blueprints/Buildings/ZeuS_Building.Zeus_Building_C"))
  (for _array_element _outactors
    (LocalVariables|SetTotalPopulation (+ (Variables|/Game/Blueprints/Buildings/ZeuS_Building.Zeus_Building_C|GetMaxResidents _array_element) (LocalVariables|GetTotalPopulation))))
  (return (LocalVariables|GetTotalPopulation)))

(fn RemainingHousing
  (bind _total_housing (CallFunction|HousingCapacity))
  (bind _current_population (CallFunction|CurrentPopulation))
  (return (- _total_housing _current_population)))

(fn CurrentPopulation
  (bind _returnvalue (CallFunction|HomelessPopulation))
  (LocalVariables|SetPopulation (+ (LocalVariables|GetPopulation) _returnvalue 0))
  (bind _outactors (Actor|GetAllActorsOfClass "/Game/Blueprints/Buildings/ZeuS_Building.Zeus_Building_C"))
  (for _array_element _outactors
    (LocalVariables|SetPopulation (+ (Variables|/Game/Blueprints/Buildings/ZeuS_Building.Zeus_Building_C|GetResidents _array_element) (LocalVariables|GetPopulation))))
  (return (LocalVariables|GetPopulation)))

(fn HomelessPopulation
  (bind _outactors (Actor|GetAllActorsOfClass "/Game/Blueprints/Pawns/Zeus_Immigrant.Zeus_Immigrant_C"))
  (return (Utilities|Array|Length _outactors)))