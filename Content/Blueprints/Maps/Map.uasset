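; Map actor that procedurally builds a square grid of tiles and scatters trees across it.
; GenerateMap spawns MapSize squared tiles row by row at TileSize spacing, adding trees at a tile's TreePlacement point and marking it occupied where noise exceeds a threshold.
; GetNoiseAtLocation samples fixed-seed simplex noise through a scale-bias module at grid coordinates, creating new noise modules on each call.
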(event EventBeginPlay)

(event Collision|EventActorBeginOverlap
  (params (OtherActor :type Actor%20Object%20Reference)))

(event EventTick
  (params (DeltaSeconds :type Float%20%28single-precision%29)))

(fn ConstructionScript)

(fn GenerateMap
  (params (MapSize :type Integer))
  (for _index (range 1 (* MapSize MapSize))
    (bind _returnvalue (Game|SpawnActorfromClass "/Game/Blueprints/Tiles/Tile.Tile_C" (Math|Transform|MakeTransform (Math|Vector|MakeVector (Math|Conversions|ToFloat(Integer) (* (LocalVariables|Getx) (Variables|Default|GetTileSize))) (Math|Conversions|ToFloat(Integer) (* (LocalVariables|Gety) (Variables|Default|GetTileSize))) 0.0)) "Undefined" 0 0))
    (bind _returnvalue_2 (CallFunction|GetNoiseatLocation (LocalVariables|Getx) (LocalVariables|Gety)))
    (if (> _returnvalue_2 0.5)
      (Game|SpawnActorfromClass "/Game/Blueprints/Buildings/Zeus_Trees.Zeus_Trees_C" (Math|Transform|MakeTransform (Transformation|GetWorldLocation (Variables|/Game/Blueprints/Tiles/Tile.Tile_C|GetTreePlacement _returnvalue))) "Undefined" _returnvalue 0)
      (Variables|/Game/Blueprints/Tiles/Tile.Tile_C|SetOccupied _returnvalue true))
    (Math|Integer|IncrementInt (LocalVariables|Getx)
      (:%20%20
        (if (== (LocalVariables|Getx) MapSize)
          (Math|Integer|IncrementInt (LocalVariables|Gety)
            (:%20%20
              (LocalVariables|Setx 0))))))))

(fn GetNoiseatLocation
  (params (X :type Integer) (Y :type Integer))
  (bind _self self)
  (bind _returnvalue (Class|UFNNoiseGenerator|GetNoise2D (Class|UFNBlueprintFunctionLibrary|CreateScaleBiasModule _self (Class|UFNBlueprintFunctionLibrary|CreateSimpleNoiseGenerator _self "SimpleSimplex" 420 0.1 "InterpLinear" "None" 3e+01) 1e+01 0.0) (Math|Conversions|ToFloat(Integer) X) (Math|Conversions|ToFloat(Integer) Y)))
  (return _returnvalue))