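; GodController is a player controller Blueprint that uses the mouse wheel to shift the height of the player character's movement plane.
; Each non-zero MouseWheelAxis value moves the movement component's plane constraint origin up or down by a fixed Z step, based on scroll direction alone.
; The plane constraint itself is not enabled or configured here, and the other events and construction script are empty.
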(event EventBeginPlay)

(event EventTick
  (params (DeltaSeconds :type Float%20%28single-precision%29)))

(event Input|MouseEvents|MouseWheelAxis
  (params (AxisValue :type Float%20%28single-precision%29))
  (bind _returnvalue (Game|GetPlayerCharacter 0))
  (bind _returnvalue_2 (Game|GetPlayerCharacter 0))
  (bind _returnvalue_3 (Pawn|GetMovementComponent _returnvalue))
  (bind _returnvalue_4 (Pawn|GetMovementComponent _returnvalue_2))
  (if (!= AxisValue 0.0)
    (if (> AxisValue 0.0)
      (Class|MovementComponent|SetPlaneConstraintOrigin _returnvalue_4 (+ (Class|MovementComponent|GetPlaneConstraintOrigin _returnvalue_4) "0, 0,100.000000"))
      (else
        (Class|MovementComponent|SetPlaneConstraintOrigin _returnvalue_3 (+ (Class|MovementComponent|GetPlaneConstraintOrigin _returnvalue_3) "0, 0,-100.000000"))))))

(event Input|MouseEvents|MouseWheelUp
  (params (Key :type Key%20Structure :default "AnyKey")))

(fn ConstructionScript)