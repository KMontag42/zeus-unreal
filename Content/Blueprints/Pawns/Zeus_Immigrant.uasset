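; Immigrant pawn that walks to the nearest available building, adds itself as a resident and is then destroyed.
; Tick polls GetClosestHouse until it returns a valid target, then starts AI MoveTo and sets Seeking, which is never cleared on failure.
; GetClosestHouse scans all Zeus_Building actors, using synchronous pathfinding to reject partial paths among closer candidates.
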(event EventBeginPlay)

(event Collision|EventActorBeginOverlap
  (params (OtherActor :type Actor%20Object%20Reference)))

(event EventTick
  (params (DeltaSeconds :type Float%20%28single-precision%29))
  (if (not (Variables|Default|GetSeeking))
    (bind _closestbuilding (CallFunction|GetClosestHouse))
    (Utilities|IsValid _closestbuilding
      (:Is%20Valid
        (AI|AIMoveTo self "0, 0, 0" _closestbuilding 1e+01 false
          (:then
            (Variables|Default|SetSeeking true))
          (:OnSuccess
            (Math|Integer|IncrementInt (Variables|/Game/Blueprints/Buildings/ZeuS_Building.Zeus_Building_C|GetResidents _closestbuilding)
              (:%20%20
                (Actor|DestroyActor)))))))))

(fn ConstructionScript)

(fn GetClosestHouse
  (bind _outactors (Actor|GetAllActorsOfClass "/Game/Blueprints/Buildings/ZeuS_Building.Zeus_Building_C"))
  (for _array_element _outactors
    (bind _available (Default|IsAvailable _array_element))
    (if _available
      (if (< (Transformation|GetDistanceTo self _array_element) (LocalVariables|GetClosestDistance))
        (bind _returnvalue (Class|NavigationSystem|FindPathtoActorSynchronously (Transformation|GetActorLocation) _array_element 5e+01 self))
        (if (not (Class|NavigationPath|IsPartial _returnvalue))
          (LocalVariables|SetCurrentClosest _array_element)
          (LocalVariables|SetClosestDistance (Transformation|GetDistanceTo self _array_element))))))
  (return (LocalVariables|GetCurrentClosest)))