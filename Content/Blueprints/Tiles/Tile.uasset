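; Clickable grass tile for placing houses in a Zeus god game, active when the controller's cursor state is House.
; Hovering spawns a collision-free preview building and tints footprint tiles red or blue by occupancy via a dynamic material; leaving removes both.
; Clicking spawns a basic house if all footprint tiles are free, then marks them occupied.
; A diagonal box trace from the tile finds that footprint for every check.
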(event EventBeginPlay)

(event Collision|EventActorBeginOverlap
  (params (OtherActor :type Actor%20Object%20Reference)))

(event EventTick
  (params (DeltaSeconds :type Float%20%28single-precision%29)))

(event MouseInput|EventActorBeginCursorOver
  (bind _aszeus_god_controller (Utilities|Casting|CastToZeus_GodController (Game|GetPlayerController 0)))
  (switch Utilities|FlowControl|Switch|SwitchonCursorStates (Variables|/Game/Blueprints/PlayerControllers/Zeus_GodController.Zeus_GodController_C|GetCurrentCursorState _aszeus_god_controller)
    (:NewEnumerator1
      (CallFunction|SpawnHoverBuilding "/Game/Blueprints/Buildings/Zeus_HouseBuilding_Complete.Zeus_HouseBuilding_Complete_C"))))

(event MouseInput|EventActorOnClicked
  (params (ButtonPressed :type Key%20Structure :default "AnyKey"))
  (bind _aszeus_god_controller (Utilities|Casting|CastToZeus_GodController (Game|GetPlayerController 0)))
  (switch Utilities|FlowControl|Switch|SwitchonCursorStates (Variables|/Game/Blueprints/PlayerControllers/Zeus_GodController.Zeus_GodController_C|GetCurrentCursorState _aszeus_god_controller)
    (:NewEnumerator1
      (bind _value (CallFunction|AllNeighborsAvailable))
      (if _value
        (CallFunction|Buildon "/Game/Blueprints/Buildings/Zeus_HouseBuilding_Basic.Zeus_HouseBuilding_Basic_C")))))

(event MouseInput|EventActorEndCursorOver
  (Utilities|IsValid (Variables|Default|GetHoveredBuilding)
    (:Is%20Valid
      (Actor|DestroyActor (Variables|Default|GetHoveredBuilding))
      (CallFunction|ResetNeighborColors))))

(fn ConstructionScript
  (bind _returnvalue (Rendering|Material|CreateDynamicMaterialInstance "/Game/Assets/Zeus_Grass_Inst.Zeus_Grass_Inst" :!class /Script/Engine.KismetMaterialLibrary))
  (Rendering|Material|SetMaterial (Variables|Debug|GetStaticMeshComponent) 0 _returnvalue)
  (Variables|Default|SetOriginalMaterial _returnvalue))

(fn CheckNeighborsforOccupied
  (bind _hittiles (CallFunction|GetNeighbors "ObjectTypeQuery1"))
  (for _array_element _hittiles
    (if (Variables|Tile_C|GetOccupied _array_element)
      (CallFunction|SetColor _array_element "(R=1.000000,G=0.000000,B=0.000000,A=1.000000)")
      (else
        (CallFunction|SetColor _array_element "(R=0.000000,G=0.004799,B=1.000000,A=1.000000)")))))

(fn SetColor
  (params (Color :type Linear%20Color%20Structure))
  (Rendering|Material|SetVectorParameterValue (Variables|Default|GetOriginalMaterial) "Color" Color :!class /Script/Engine.MaterialInstanceDynamic))

(fn GetNeighbors
  (params (Type :type EObjectTypeQuery%20Enum))
  (bind (_outhits _returnvalue) (Class|KismetSystemLibrary|BoxTraceMultiforObjects (Transformation|GetActorLocation) (+ (Transformation|GetActorLocation) "100.000000,100.000000,0.000000") "10.000000,10.000000,10.000000" "0, 0,0.000000" (Utilities|Array|MakeArray Type) false 0 "None" false))
  (for _array_element _outhits
    (bind _astile (Utilities|Casting|CastToTile (.HitActor (Collision|BreakHitResult _array_element))))
    (Utilities|Array|AddUnique (LocalVariables|GetTiles) _astile))
  (return _outhits _returnvalue (LocalVariables|GetTiles)))

(fn ResetNeighborColors
  (bind _hittiles (CallFunction|GetNeighbors "ObjectTypeQuery1"))
  (for _array_element _hittiles
    (CallFunction|SetColor _array_element "(R=1.000000,G=1.000000,B=1.000000,A=1.000000)")))

(fn SpawnHoverBuilding
  (params (Class :type Actor%20Class%20Reference))
  (bind _returnvalue (Game|SpawnActorfromClass Class (Math|Conversions|ToTransform(Vector) (+ (Transformation|GetWorldLocation (Variables|Default|GetBuildingPlacement)) "0, 0,50.000000")) "Undefined" 0 0))
  (bind _asstatic_mesh_actor (Utilities|Casting|CastToStaticMeshActor _returnvalue))
  (Variables|Default|SetHoveredBuilding _returnvalue)
  (Collision|SetCollisionEnabled (Variables|/Script/Engine.StaticMeshActor|GetStaticMeshComponent _asstatic_mesh_actor) "NoCollision")
  (CallFunction|CheckNeighborsforOccupied))

(fn Buildon
  (params (Class :type Actor%20Class%20Reference))
  (bind _returnvalue (Game|SpawnActorfromClass Class (Math|Conversions|ToTransform(Vector) (+ (Transformation|GetWorldLocation (Variables|Default|GetBuildingPlacement)) "0, 0,50.000000")) "Undefined" 0 0))
  (bind _hittiles (CallFunction|GetNeighbors "ObjectTypeQuery1"))
  (for _array_element _hittiles
    (Variables|Tile_C|SetOccupied _array_element true))
  (return _returnvalue))

(fn AllNeighborsAvailable
  (bind _hittiles (CallFunction|GetNeighbors "ObjectTypeQuery1"))
  (for _array_element _hittiles
    (LocalVariables|SetAllAvailable (and (LocalVariables|GetAllAvailable) (not (Variables|Tile_C|GetOccupied _array_element)))))
  (return (LocalVariables|GetAllAvailable)))